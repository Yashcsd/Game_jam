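; BPC_health is a health component in the enemy ANT folder that tracks a Health value and handles death.
; IncreaseHealth adds to Health with a 0–100 clamp, while DecreaseHealth subtracts damage without clamping; both then call UpdatedHealth.
; When damage brings Health to zero or below, it calls Dead and immediately opens level_1 by name, so level loading is hard-wired into the component.
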(fn `Decrease_health`
  (params (Damage :type "Float (double-precision)"))
  (set `self.health` (- (`self.health`) Damage))
  (`self.Updated_health`)
  (if (<= (`self.health`) 0.0)
    (`self.Dead`)
    (`GameplayStatics.OpenLevel` "level_1")))

(fn `Increase_health`
  (params (Amount :type "Float (double-precision)"))
  (set `self.health` (`KismetMathLibrary.FClamp` (+ (`self.health`) Amount) 0.0 100.0))
  (`self.Updated_health`))