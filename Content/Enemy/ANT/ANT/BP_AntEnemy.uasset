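; BP_AntEnemy is an ant enemy that chases the player character and attacks on arrival.
; PawnSensing sets IsSeePlayer on seeing any pawn and starts an AI MoveTo toward player 0.
; A successful move plays the attack montage, followed by a short delay.
; Tick halts movement until the first sighting; the branch that would clear the flag is unreachable, and CanAttack never gates the attack.
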(event `self.ReceiveTick`
  (params (DeltaSeconds :type "Float (single-precision)"))
  (if (not (`self.IsSeePlayer?`))
    (`MovementComponent.StopMovementImmediately` (`self.CharacterMovement`))))

(event `self.PawnSensing.OnSeePawn`
  (params (Pawn :type "Pawn Object Reference"))
  (set `self.IsSeePlayer?` true)
  (`self.FollowPlayer`))

(event `FollowPlayer`
  (set `self.CanAttack?` true)
  (if (`self.IsSeePlayer?`)
    (`|AIMoveTo` self (0.0 0.0 0.0) (`GameplayStatics.GetPlayerCharacter` 0) 70.0
      (:`OnSuccess`
        (set `self.CanAttack?` (`self.CanAttack?`))
        (if true
          (`self.PlayAnimMontage` "/Game/Enemy/Animation/AM_Ant_Attack.AM_Ant_Attack")
          (`KismetSystemLibrary.Delay` 0.2)
          (set `self.CanAttack?` true)
          (else
            (set `self.IsSeePlayer?` false)))))))

(fn `UserConstructionScript`)