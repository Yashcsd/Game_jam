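; Ant enemy that pursues the player on sight and deals damage on contact.
; PawnSensing sets a seen-player flag, which is never cleared here, and calls FollowPlayer to issue an AI MoveTo targeting the first player character.
; Overlapping the Body_field component applies fixed damage to the third-person character, with no repeat while the overlap lasts.
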(event `self.body_field.OnComponentBeginOverlap`
  (params (OverlappedComponent :type "PrimitiveComponent Object Reference") (OtherActor :type "Actor Object Reference") (OtherComp :type "PrimitiveComponent Object Reference") (OtherBodyIndex :type Integer) (bFromSweep :type Boolean) (SweepResult :type "HitResult Structure (by ref)"))
  (bind _asbp_third_person_character (cast `/Game/ThirdPerson/Blueprints/BP_ThirdPersonCharacter` OtherActor))
  (`GameplayStatics.ApplyDamage` _asbp_third_person_character 20.0 null self))

(event `self.PawnSensing.OnSeePawn`
  (params (Pawn :type "Pawn Object Reference"))
  (set `self.IsSeelingPlayer?` true)
  (`self.FollowPlayer`))

(event `FollowPlayer`
  (if (`self.IsSeelingPlayer?`)
    (`|AIMoveTo` (stale `self.PawnSensing.OnSeePawn` Pawn) (0.0 0.0 0.0) (`GameplayStatics.GetPlayerCharacter` 0))))

(fn `UserConstructionScript`)